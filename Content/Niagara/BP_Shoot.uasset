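; BP_Shoot is a fired web projectile actor that trails a beam effect and stops on impact.
; On BeginPlay it launches the Projectile component along the actor's forward vector with a velocity-change impulse.
; Tick feeds the projectile's world location into the Web effect's BeamEnd parameter so the beam follows it.
; The first hit disables the projectile's physics and collision, freezing it and the beam end in place.
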(event OnComponentHit(Projectile)
  (params (HitComponent :type Primitive%20Component%20Object%20Reference) (OtherActor :type Actor%20Object%20Reference) (OtherComp :type Primitive%20Component%20Object%20Reference) (NormalImpulse :type Vector :default "0, 0, 0") (Hit :type Hit%20Result%20Structure%20%28by%20ref%29))
  (bind _projectile (Variables|Default|GetProjectile))
  (Utilities|FlowControl|DoOnce false
    (:Completed
      (Physics|SetSimulatePhysics _projectile false)
      (Collision|SetCollisionEnabled _projectile "NoCollision"))))

(event EventBeginPlay
  (Physics|AddImpulse (Variables|Default|GetProjectile) (* (Transformation|GetActorForwardVector) 3e+03) "None" true))

(event Collision|EventActorBeginOverlap
  (params (OtherActor :type Actor%20Object%20Reference)))

(event EventTick
  (params (DeltaSeconds :type Float%20%28single-precision%29))
  (Effects|Components|ParticleSystem|SetVectorParameter (Variables|Default|GetWeb) "BeamEnd" (Transformation|GetWorldLocation (Variables|Default|GetProjectile))))

(fn ConstructionScript)